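; BP_SerialManager is a manager that links a serial COM port device to a chest in the game.
; On BeginPlay it opens a fixed COM port and stores the connection.
; Each Tick it reads and prints a line from that connection, calling OpenChest on the referenced chest whenever a read succeeds, regardless of the line's content.
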(event `self.ReceiveBeginPlay`
  (bind (_bopened _returnvalue) (`SerialCom.OpenComPort` 5))
  (`KismetSystemLibrary.PrintString` (`KismetSystemLibrary.GetDisplayName` _returnvalue))
  (set `self.SerialConnection` _returnvalue))

(event `self.ReceiveTick`
  (params (DeltaSeconds :type "Float (single-precision)"))
  (bind (_bsuccess _returnvalue) (`SerialCom.Readln` (`self.SerialConnection`)))
  (`KismetSystemLibrary.PrintString` _returnvalue)
  (if _bsuccess
    (`/Game/Chest/Chest.OpenChest` (`self.ChestRef`))))

(fn `UserConstructionScript`)